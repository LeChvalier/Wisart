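; Freezable actor that drives a Dissolve effect on its Cube's materials from a clamped freeze value.
; Each AddFreeze call lowers the value at twice the delta-time rate, while Tick steadily raises it back.
; Both events write the value to the Dissolve scalar parameter, so freezing reverses gradually once calls stop.
; AddFreeze scales by frame time, which suggests per-frame calls from outside this graph.
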(event `AddFreeze`
  (bind _output_get (set `self.FreezeVal` (`KismetMathLibrary.FClamp` (- (`self.FreezeVal`) (* 2 (`GameplayStatics.GetWorldDeltaSeconds`))) -1.0 2.0)))
  (`MeshComponent.SetScalarParameterValueOnMaterials` (`self.Cube`) "Dissolve" _output_get))

(event `self.ReceiveTick`
  (params (DeltaSeconds :type "Float (single-precision)"))
  (bind _output_get (set `self.FreezeVal` (`KismetMathLibrary.FClamp` (+ (`self.FreezeVal`) (`GameplayStatics.GetWorldDeltaSeconds`)) -1.0 2.0)))
  (`MeshComponent.SetScalarParameterValueOnMaterials` (`self.Cube`) "Dissolve" _output_get))

(fn `UserConstructionScript`)