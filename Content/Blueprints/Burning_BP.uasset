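; Burning actor that can catch fire, spread it to nearby Burning_BP actors, and be frozen.
; SetOnFire and StopFire toggle two Niagara effects; AddFreeze lowers a freeze value that recovers on Tick, driving a dynamic material's Dissolve parameter.
; After a short burn, Tick extinguishes iced actors or others at random, and randomly ignites neighbors through a sphere trace.
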(event `self.ReceiveBeginPlay`
  (bind _returnvalue (`PrimitiveComponent.CreateDynamicMaterialInstance` (`self.Cube`) 0 null "None"))
  (`PrimitiveComponent.SetMaterial` (`self.Cube`) 0 _returnvalue)
  (set `self.Mat` _returnvalue))

(event `AddFreeze`
  (bind _output_get (set `self.FreezeVal` (`KismetMathLibrary.FClamp` (- (`self.FreezeVal`) (* (`GameplayStatics.GetWorldDeltaSeconds`) 2.0)) -1.0 2.0)))
  (`MaterialInstanceDynamic.SetScalarParameterValue` (`self.Mat`) "Dissolve" _output_get))

(event `StopFire`
  (set `self.IsOnFire` false)
  (`ActorComponent.Deactivate` (`self.Niagara`))
  (`ActorComponent.Deactivate` (`self.Niagara1`)))

(event `SetOnFire`
  (set `self.IsOnFire` true)
  (set `self.TimeOnFire` 0.0)
  (`ActorComponent.Activate` (`self.Niagara`) false)
  (`ActorComponent.Activate` (`self.Niagara1`) false))

(event `self.ReceiveTick`
  (params (DeltaSeconds :type "Float (single-precision)"))
  (bind _returnvalue (`self.K2_GetActorLocation`))
  (`|ExecutionSequence`
    (:`then_0`
      (set `self.TimeOnFire` (+ (`self.TimeOnFire`) DeltaSeconds))
      (if (> (`self.FreezeVal`) 1.5)
        (set `self.IsOnIce` false)
        (else
          (set `self.IsOnIce` true))))
    (:`then_1`
      (bind _output_get (set `self.FreezeVal` (`KismetMathLibrary.FClamp` (+ (`self.FreezeVal`) (* (`GameplayStatics.GetWorldDeltaSeconds`) 0.6)) -1.0 2.0)))
      (`MaterialInstanceDynamic.SetScalarParameterValue` (`self.Mat`) "Dissolve" _output_get))
    (:`then_2`
      (if (`self.IsOnFire`)
        (if (not (< (`self.TimeOnFire`) 2.0))
          (`|ExecutionSequence`
            (:`then_0`
              (if (`self.IsOnIce`)
                (`self.StopFire`)
                (elif (< (`KismetMathLibrary.RandomFloatInRange` 0.0 100000.0) 100.0)
                  (`self.StopFire`))))
            (:`then_1`
              (if (< (`KismetMathLibrary.RandomFloatInRange` 0.0 100000.0) 400.0)
                (bind _outhits (`KismetSystemLibrary.SphereTraceMulti` _returnvalue _returnvalue 300.0 "TraceTypeQuery1"))
                (for _array_element _outhits
                  (bind _asburning_bp (cast `/Game/Blueprints/Burning_BP` (`.HitActor` (`GameplayStatics.BreakHitResult` _array_element))))
                  (`self.SetOnFire` _asburning_bp))))))))))

(fn `UserConstructionScript`)